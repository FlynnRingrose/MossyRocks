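; Game mode for Mossy that runs a level countdown and handles level changes.
; BeginPlay enables the timer, and Tick feeds a one-second Delay that throttles the decrement of RemainingTime.
; Reaching zero opens the Menu level.
; While TimerEnabled is false, which nothing here sets, Tick increments NextLevelInt and opens that entry from LevelArray.
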(event `self.ReceiveBeginPlay`
  (set `self.bTimerEnabled` true))

(event `self.ReceiveTick`
  (params (DeltaSeconds :type "Float (single-precision)"))
  (if (`self.bTimerEnabled`)
    (`KismetSystemLibrary.Delay` 1.0)
    (set `self.RemainingTime` (- (`self.RemainingTime`) 1))
    (if (== 0 (`self.RemainingTime`))
      (`GameplayStatics.OpenLevel` "Menu"))
    (else
      (bind _result (`/Engine/EditorBlueprintResources/StandardMacros.IncrementInt` (`self.NextLevelInt`))
        (:`  `
          (`GameplayStatics.OpenLevel` (`|GetArrayItem` (`self.LevelArray`) _result)))))))

(fn `UserConstructionScript`)
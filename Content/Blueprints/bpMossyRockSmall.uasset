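; Small mossy rock actor that animates into place when play begins and responds to a victory sequence.
; One second after BeginPlay, a timeline slides the actor along negative world X from its spawn location while blending the Rock component toward a preset rotation.
; The captured start rotation is world-space but is applied as relative rotation.
; VictorySequence instantly raises the actor along Z from its current location.
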(event `self.ReceiveTick`
  (params (DeltaSeconds :type "Float (single-precision)")))

(event `self.ReceiveBeginPlay`
  (bind _spawnlocation (`self.SpawnLocation`))
  ;[1 1 1] Spawn Animation
  (`KismetSystemLibrary.Delay` 1.0)
  (set `self.SpawnLocation` (`self.K2_GetActorLocation`))
  (set `self.SpawnRotation` (`SceneComponent.K2_GetComponentRotation` (`self.Rock`)))
  (bind (_direction _spawn) (`Timeline|SpawnAnimation`)
    (:`Update`
      (`self.K2_SetActorLocation` (`KismetMathLibrary.VLerp` _spawnlocation (+ _spawnlocation (-300.0 0.0 0.0)) _spawn))
      (`SceneComponent.K2_SetRelativeRotation` (`self.Rock`) (`KismetMathLibrary.RLerp` (`self.SpawnRotation`) (`self.ChrissMagicNumberJudgment`) _spawn) false false))))

(event `self.VictorySequence`
  (bind _output_get (set `self.CurrentLocation` (`self.K2_GetActorLocation`)))
  (`self.K2_SetActorLocation` (+ _output_get (0.0 0.0 500.0))))

(fn `UserConstructionScript`)